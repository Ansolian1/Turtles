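; Turtle3 is a turtle actor Blueprint that alternates its Destination between its spawn location and TargetPoint.
; BeginPlay runs the parent logic, caches StartPosition, then enters a looping chain of two unequal Delays that switches Destination.
; The loop checks IsFinishing after each switch to TargetPoint, so it ends with that point as the Destination.
; This graph only sets Destination and contains no movement code.
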(event EventBeginPlay
  ;[1 1 1] Cash start position
  (|CallParentFunction)
  (Variables|Default|SetStartPosition (Transformation|GetActorLocation))
  ;[1 1 1] ChangingDestination
  (Utilities|FlowControl|Delay 1.0 :!label _label)
  (Variables|Default|SetDestination (Variables|Default|GetStartPosition))
  (Utilities|FlowControl|Delay 0.5)
  (Variables|Default|SetDestination (Variables|Default|GetTargetPoint))
  (if (not (Variables|Default|GetIsFinishing))
    (goto _label)))

(fn ConstructionScript
  (|CallParentFunction))