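; Parent Blueprint for an AI-moved turtle that travels to a target point and celebrates on arrival.
; BeginPlay copies the target into the destination, and Tick reissues a simple move to it through the AI controller every frame.
; Tick also checks distance to the target; once within a small radius, a one-time flag gates playing the finish effect, activating sparks and stopping the footsteps.
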(event EventBeginPlay
  ;[1 1 1] Destination set
  (Variables|Default|SetDestination (Variables|Components|GetTargetPoint)))

(event EventTick
  (params (DeltaSeconds :type Float%20%28single-precision%29))
  ;[1 1 1] Moving
  (AI|Navigation|SimpleMovetoLocation (AI|GetAIController self) (Variables|Default|GetDestination))
  ;[1 1 1] Check finishing
  (if (not (Variables|Default|GetIsFinishing))
    (if (<= (Math|Vector|VectorLength (- (Transformation|GetActorLocation) (Variables|Components|GetTargetPoint))) 1e+02)
      ;[1 1 1] Finishing
      (Audio|Components|Audio|Play (Variables|Default|GetFinish) 0.0)
      (Components|Activation|Activate (Variables|Default|GetP_Sparks) false)
      (Variables|Default|SetIsFinishing true)
      (Audio|Components|Audio|Stop (Variables|Default|GetSteps)))))

(fn ConstructionScript)