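; Turtle2 is a turtle character Blueprint that moves in a stop-and-go rhythm.
; BeginPlay runs the parent logic, then caches the CharacterMovement walk speed as DefaultSpeed.
; An endless Delay loop alternates a longer moving phase with a shorter pause by zeroing and restoring MaxWalkSpeed.
; The graph issues no movement input of its own and only modulates speed.
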(event EventBeginPlay
  (bind _charactermovement (Variables|Character|GetCharacterMovement))
  ;[1 1 1] Cash default speed
  (|CallParentFunction)
  (Variables|Default|SetDefaultSpeed (Variables|/Script/Engine.CharacterMovementComponent|GetMaxWalkSpeed (Variables|Character|GetCharacterMovement)))
  ;[1 1 1] Moving&Stopping
  (Utilities|FlowControl|Delay 1.0 :!label _label)
  (Variables|/Script/Engine.CharacterMovementComponent|SetMaxWalkSpeed _charactermovement 0.0)
  (Utilities|FlowControl|Delay 0.5)
  (Variables|/Script/Engine.CharacterMovementComponent|SetMaxWalkSpeed _charactermovement (Variables|Default|GetDefaultSpeed))
  (goto _label))

(fn ConstructionScript
  (|CallParentFunction))